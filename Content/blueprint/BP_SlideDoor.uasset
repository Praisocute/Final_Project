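; BP_SlideDoor is a two-panel sliding door that opens only after enough items have been collected.
; Collect increments a counter, and entering the Box trigger plays a timeline that slides Left and Right apart once the count reaches MaxItemCollect.
; Leaving the trigger reverses the timeline.
; OpenDoorChack repeats the count check and calls BoxOverlapComponent on the trigger through a DoOnce, without directly driving the timeline.
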(event `self.Box.OnComponentBeginOverlap`
  (params (OverlappedComponent :type "PrimitiveComponent Object Reference") (OtherActor :type "Actor Object Reference") (OtherComp :type "PrimitiveComponent Object Reference") (OtherBodyIndex :type Integer) (bFromSweep :type Boolean) (SweepResult :type "HitResult Structure (by ref)"))
  (if (>= (`self.currentItenCollect`) (`self.MaxItemCollect`))
    (bind (_direction _door_track) (`Timeline|Timeline` :!label _label)
      (:`Update`
        (`SceneComponent.K2_SetRelativeLocation` (`self.Left`) (`KismetMathLibrary.MakeVector` (`KismetMathLibrary.Lerp` -18.0 70.0 _door_track) 0.0 0.0) false false)
        (`SceneComponent.K2_SetRelativeLocation` (`self.Right`) (`KismetMathLibrary.MakeVector` (`KismetMathLibrary.Lerp` -179.0 -271.0 _door_track) 0.0 0.0) false false)))))

(event `self.Box.OnComponentEndOverlap`
  (params (OverlappedComponent :type "PrimitiveComponent Object Reference") (OtherActor :type "Actor Object Reference") (OtherComp :type "PrimitiveComponent Object Reference") (OtherBodyIndex :type Integer))
  (goto _label :!via `Reverse`))

(event `Collect`
  (`/Engine/EditorBlueprintResources/StandardMacros.IncrementInt` (`self.currentItenCollect`)))

(event `Open Door Chack`
  (if (>= (`self.currentItenCollect`) (`self.MaxItemCollect`))
    (`/Engine/EditorBlueprintResources/StandardMacros.DoOnce` false
      (:`Completed`
        (`PrimitiveComponent.K2_BoxOverlapComponent` :`self` (`self.Box`))))))

(fn `UserConstructionScript`)