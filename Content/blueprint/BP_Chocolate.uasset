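; BP_Chocolate is an AI pawn that wanders between random tagged actors and chases the player character when it perceives one.
; Patrol starts at BeginPlay, moving to a random tagged actor and repeating after a short pause on success.
; AI Perception updates raise walk speed and move it toward the player, without checking whether the stimulus was gained or lost.
; Forgetting the player lowers speed and resumes patrol.
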(event `self.ReceiveBeginPlay`
  (add `AIPerceptionComponent.OnTargetPerceptionForgotten` (`self.AIPerception`) (delegate `OnTargetPerceptionForgotten_Event`))
  (bind _outactors (`GameplayStatics.GetAllActorsWithTag` (`self.Tag`) :!label _label))
  (`|AIMoveTo` self (0.0 0.0 0.0) (`KismetArrayLibrary.Array_Random` _outactors)
    (:`OnSuccess`
      (`KismetSystemLibrary.Delay` 1.5)
      (goto _label))))

(event `OnTargetPerceptionForgotten_Event`
  (params (Actor :type "Actor Object Reference")))

(event `self.AIPerception.OnTargetPerceptionForgotten`
  (params (Actor :type "Actor Object Reference"))
  (cast `/Game/ThirdPerson/Blueprints/BP_ThirdPersonCharacter` Actor)
  (set `CharacterMovementComponent.MaxWalkSpeed` 300.0 (`self.CharacterMovement`))
  (goto _label))

(event `self.AIPerception.OnTargetPerceptionUpdated`
  (params (Actor :type "Actor Object Reference") (Stimulus :type "AIStimulus Structure"))
  (bind _asbp_third_person_character (cast `/Game/ThirdPerson/Blueprints/BP_ThirdPersonCharacter` Actor))
  (set `CharacterMovementComponent.MaxWalkSpeed` 450.0 (`self.CharacterMovement`))
  (`|AIMoveTo` self (0.0 0.0 0.0) _asbp_third_person_character))

(fn `UserConstructionScript`)